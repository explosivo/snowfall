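; Heart item actor that spins and bobs in place as a visual effect, with no pickup logic of its own.
; A Rotate timeline starts on BeginPlay and feeds its Yaw track to Spin, which sets the actor rotation, and its Theta track to Bounce.
; Bounce adds half the sine of Theta to the current Z on every update, so the vertical offset accumulates per frame rather than following a stored base height.
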(event `self.ReceiveBeginPlay`
  (bind (_direction _yaw _theta) (`Timeline|Rotate` :!via `PlayFromStart`)
    (:`Update`
      (`self.Spin` _yaw)
      (`self.Bounce` _theta))))

(fn `Bounce`
  (params (Theta :type "Float (double-precision)"))
  (`self.K2_SetActorLocation` (`KismetMathLibrary.MakeVector` (.x (`self.K2_GetActorLocation`)) (.y (`self.K2_GetActorLocation`)) (+ (.z (`self.K2_GetActorLocation`)) (/ (`KismetMathLibrary.Sin` Theta) 2.0)))))

(fn `Spin`
  (params (Yaw :type "Float (double-precision)"))
  (`self.SetActorRotation` (`KismetMathLibrary.MakeRotator` 0.0 0.0 Yaw)))

(fn `UserConstructionScript`)